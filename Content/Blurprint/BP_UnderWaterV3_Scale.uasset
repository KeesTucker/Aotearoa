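; An underwater environment actor that sets up the post-process look, ocean surface and caustics lighting from its variables.
; The construction script writes color grading, LUT, blur, chromatic aberration, exposure, vignette and post-process materials into the PostProcess component.
; It also applies visibility and material to the ocean surface mesh.
; Caustics come from a light with configurable color, intensity and visibility, patterned by a light function material.
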(fn `UserConstructionScript`
  (locals (`Cos color` :type "LinearColor Structure" :default (struct :`R` 0.524927 :`G` 0.879212 :`B` 1.0)))
  (bind _caustics_light (`self.Caustics Light`))
  (bind _sm_oceansurface (`self.SM_OceanSurface`))
  (bind (_saturation _contrast _gamma _gain _offset) (break `ColorGradePerRangeSettings` (`self.Color Grade Settings`)))
  (setmembers `PostProcessSettings` :`StructRef` (`PostProcessComponent.Settings` (`self.PostProcess`)) :`BloomMethod` "BM_FFT" :`WhiteTemp` (`self.Temp`) :`WhiteTint` (`self.Tint`) :`ColorSaturation` _saturation :`ColorContrast` _contrast :`ColorGamma` _gamma :`ColorGain` _gain :`ColorOffset` _offset :`SceneFringeIntensity` (`self.Chromatic Intensity`) :`BloomIntensity` (`self.Water Blur`) :`DynamicGlobalIlluminationMethod` (`self.Reflection`) :`ReflectionMethod` (`self.Global illumination`) :`AutoExposureBias` (`self.Exposure`) :`VignetteIntensity` (`self.Vignette Intensity`) :`ColorGradingIntensity` (`self.Color Grading LUT Intensity`) :`ColorGradingLUT` (`self.Color Grading LUT`) :`WeightedBlendables` (`self.Post Process Materials`))
  (`SceneComponent.SetVisibility` _sm_oceansurface (`self.Water Visibility`) false)
  (`PrimitiveComponent.SetMaterial` _sm_oceansurface 0 (`self.Material`))
  (`LightComponent.SetLightColor` _caustics_light (`self.Caustics Color`) true)
  (`SceneComponent.SetVisibility` _caustics_light (`self.Caustics Visibility`) false)
  (`LightComponent.SetIntensity` _caustics_light (`self.Caustics Intensity`))
  (`LightComponent.SetLightFunctionMaterial` _caustics_light (`self.Caustics Material`)))